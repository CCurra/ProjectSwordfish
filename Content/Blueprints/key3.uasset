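; Key pickup actor that spins steadily around its local yaw axis every tick, scaled by delta time.
; BeginPlay binds the actor's hit event, which continues only if the other actor casts to FirstPersonCharacter.
; On such a hit it increases the character's float Keys count using integer math, prints the new total and destroys itself.
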(event Custom|OnActorHit_Event_0
  (params (SelfActor :type Actor%20Object%20Reference) (OtherActor :type Actor%20Object%20Reference) (NormalImpulse :type Vector) (Hit :type Hit%20Result%20Structure%20%28by%20ref%29))
  ;[1 1 1] When character picks up key, set var "keys_obtained" relative to 1
  (bind _asfirst_person_character (Utilities|Casting|CastToFirstPersonCharacter OtherActor))
  (bind _result (Math|Integer|IncrementInt (+ (Math|Float|Truncate (Variables|/Game/FirstPersonBP/Blueprints/FirstPersonCharacter.FirstPersonCharacter_C|GetKeys _asfirst_person_character)) 1))
    (:%20%20
      (bind _output_get (Variables|/Game/FirstPersonBP/Blueprints/FirstPersonCharacter.FirstPersonCharacter_C|SetKeys _asfirst_person_character (Math|Conversions|ToFloat(Integer) _result)))
      (Development|PrintString (Utilities|String|ToString(Integer) (Math|Float|Truncate _output_get)))
      (Actor|DestroyActor))))

(event EventTick
  (params (DeltaSeconds :type Float%20%28single-precision%29))
  (Variables|Default|SetYawperSecond 1.2e+02)
  (Transformation|AddActorLocalRotation (Math|Rotator|MakeRotator 0.0 0.0 (* DeltaSeconds (Variables|Default|GetYawperSecond))) false false))

(event Collision|EventActorBeginOverlap
  (params (OtherActor :type Actor%20Object%20Reference)))

(event EventBeginPlay
  ;[1 1 1] When character picks up key, set var "keys_obtained" relative to 1
  (EventDispatchers|AssignOnActorHit (delegate Custom|OnActorHit_Event_0))
  (bind _asfirst_person_character (Utilities|Casting|CastToFirstPersonCharacter (stale Custom|OnActorHit_Event_0 OtherActor)))
  (bind _result (Math|Integer|IncrementInt (+ (Math|Float|Truncate (Variables|/Game/FirstPersonBP/Blueprints/FirstPersonCharacter.FirstPersonCharacter_C|GetKeys _asfirst_person_character)) 1))
    (:%20%20
      (bind _output_get (Variables|/Game/FirstPersonBP/Blueprints/FirstPersonCharacter.FirstPersonCharacter_C|SetKeys _asfirst_person_character (Math|Conversions|ToFloat(Integer) _result)))
      (Development|PrintString (Utilities|String|ToString(Integer) (Math|Float|Truncate _output_get)))
      (Actor|DestroyActor))))

(fn ConstructionScript)