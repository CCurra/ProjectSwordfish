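; A key-locked door Blueprint that opens when a FirstPersonCharacter holding the required key type enters its overlap volume.
; On overlap, it searches the character's OwnedKeys, removes a matching key and plays a sound at TargetLocation.
; The DoorMovement timeline then lerps the static mesh's relative location from zero to TargetLocation, with no logic to close it again.
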(event OnComponentBeginOverlap(Overlay)
  (params (OverlappedComponent :type Primitive%20Component%20Object%20Reference) (OtherActor :type Actor%20Object%20Reference) (OtherComp :type Primitive%20Component%20Object%20Reference) (OtherBodyIndex :type Integer) (bFromSweep :type Boolean) (SweepResult :type Hit%20Result%20Structure%20%28by%20ref%29))
  (bind _target_location (Variables|Default|GetTarget%20Location))
  (if true
    (bind _asfirst_person_character (Utilities|Casting|CastToFirstPersonCharacter OtherActor))
    (for (_array_element _array_index) (Variables|/Game/FirstPersonBP/Blueprints/FirstPersonCharacter.FirstPersonCharacter_C|GetOwned%20Keys _asfirst_person_character)
      (if (Utilities|Enum|Equal(Enum) _array_element (Variables|Default|GetRequiredkeytype))
        (Utilities|Array|RemoveIndex (Variables|/Game/FirstPersonBP/Blueprints/FirstPersonCharacter.FirstPersonCharacter_C|GetOwned%20Keys _asfirst_person_character) _array_index)
        (Audio|PlaySoundatLocation 0 _target_location "0, 0, 0" 1.0 1.0 0.0 0 0 0)
        (bind _alpha (Timeline|DoorMovement Play)
          (:Update
            (Transformation|SetRelativeLocation (Variables|Default|GetStaticMesh) (Math|Vector|Lerp(Vector) "0, 0, 0" _target_location _alpha) false false)))))))

(fn ConstructionScript)