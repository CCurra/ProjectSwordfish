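; A double door Blueprint meant to open with a required key type held by the first-person character.
; Overlapping its trigger loops over the character's OwnedKeysDD array, but the loop body is unconnected, so nothing happens.
; The orphaned logic would match the key, call RemoveIndex twice at that index, and play a timeline that lerps the mesh to TargetLocation.
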(event OnComponentBeginOverlap(Overlay)
  (params (OverlappedComponent :type Primitive%20Component%20Object%20Reference) (OtherActor :type Actor%20Object%20Reference) (OtherComp :type Primitive%20Component%20Object%20Reference) (OtherBodyIndex :type Integer) (bFromSweep :type Boolean) (SweepResult :type Hit%20Result%20Structure%20%28by%20ref%29))
  (bind _asfirst_person_character (Utilities|Casting|CastToFirstPersonCharacter OtherActor))
  (for (_array_element _array_index) (Variables|/Game/FirstPersonBP/Blueprints/FirstPersonCharacter.FirstPersonCharacter_C|GetOwned%20Keys%20DD _asfirst_person_character)
    _))

(event Collision|EventActorBeginOverlap
  (params (OtherActor :type Actor%20Object%20Reference)))

(event EventTick
  (params (DeltaSeconds :type Float%20%28single-precision%29)))

(fn ConstructionScript)