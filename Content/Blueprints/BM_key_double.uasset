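; BM_key_double is a spinning key pickup for the double door key in the first-person game.
; Each tick it yaws at a constant rate, and the construction script sets the key mesh to a yellow material.
; On overlap with the FirstPersonCharacter it adds the same key enum entry twice to the character's OwnedKeys, then destroys itself.
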(event OnComponentBeginOverlap(Overlap)
  (params (OverlappedComponent :type Primitive%20Component%20Object%20Reference) (OtherActor :type Actor%20Object%20Reference) (OtherComp :type Primitive%20Component%20Object%20Reference) (OtherBodyIndex :type Integer) (bFromSweep :type Boolean) (SweepResult :type Hit%20Result%20Structure%20%28by%20ref%29))
  (bind _asfirst_person_character (Utilities|Casting|CastToFirstPersonCharacter OtherActor))
  (Utilities|Array|Add (Variables|/Game/FirstPersonBP/Blueprints/FirstPersonCharacter.FirstPersonCharacter_C|GetOwned%20Keys _asfirst_person_character) "NewEnumerator4")
  (Utilities|Array|Add (Variables|/Game/FirstPersonBP/Blueprints/FirstPersonCharacter.FirstPersonCharacter_C|GetOwned%20Keys _asfirst_person_character) "NewEnumerator4")
  (Actor|DestroyActor))

(event EventTick
  (params (DeltaSeconds :type Float%20%28single-precision%29))
  (Variables|Default|SetYawperSecond 1.2e+02)
  (Transformation|AddActorLocalRotation (Math|Rotator|MakeRotator 0.0 0.0 (* DeltaSeconds (Variables|Default|GetYawperSecond))) false false))

(fn ConstructionScript
  (Rendering|Material|SetMaterial (Variables|Default|GetKey) 0 (Utilities|Select :Index "NewEnumerator4" :NewEnumerator4 "/Game/Blueprints/m_yellow.m_yellow")))