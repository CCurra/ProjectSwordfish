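; A door Blueprint that opens when a FirstPersonCharacter carrying the matching key enters its Overlay trigger.
; The overlap event searches the character's OwnedKeys for one hard-coded key enum value and removes it on a match.
; A timeline then slides the StaticMesh from its relative origin to TargetLocation, with no logic to close it again.
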(event OnComponentBeginOverlap(Overlay)
  (params (OverlappedComponent :type Primitive%20Component%20Object%20Reference) (OtherActor :type Actor%20Object%20Reference) (OtherComp :type Primitive%20Component%20Object%20Reference) (OtherBodyIndex :type Integer) (bFromSweep :type Boolean) (SweepResult :type Hit%20Result%20Structure%20%28by%20ref%29))
  (bind _asfirst_person_character (Utilities|Casting|CastToFirstPersonCharacter OtherActor))
  (for (_array_element _array_index) (Variables|/Game/FirstPersonBP/Blueprints/FirstPersonCharacter.FirstPersonCharacter_C|GetOwned%20Keys _asfirst_person_character)
    (if (Utilities|Enum|Equal(Enum) _array_element "NewEnumerator4")
      (Utilities|Array|RemoveIndex (Variables|/Game/FirstPersonBP/Blueprints/FirstPersonCharacter.FirstPersonCharacter_C|GetOwned%20Keys _asfirst_person_character) _array_index)
      (bind _alpha (Timeline|Timeline_0 Play)
        (:Update
          (Transformation|SetRelativeLocation (Variables|Default|GetStaticMesh) (Math|Vector|Lerp(Vector) "0, 0, 0" (Variables|Default|GetTarget%20Location) _alpha) false false))))))

(fn ConstructionScript)